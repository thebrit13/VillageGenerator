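; Building actor Blueprint that describes a footprint in tiles through BuildingX, BuildingY and TileSize.
; DrawExtents draws a thin debug box at the actor's location, sized from those tile counts and the tile size.
; Its only call in the event graph is unconnected, and the events and construction script are empty, so the Blueprint currently runs no logic.
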(event OnLiveLinkUpdated(LiveLinkComponentController)
  (params (DeltaTime :type Float%20%28single-precision%29)))

(event EventBeginPlay)

(event Collision|EventActorBeginOverlap
  (params (OtherActor :type Actor%20Object%20Reference)))

(event EventTick
  (params (DeltaSeconds :type Float%20%28single-precision%29)))

(fn ConstructionScript)

(fn DrawExtents
  (bind _tilesize (Variables|Default|GetTileSize))
  (Rendering|Debug|DrawDebugBox :Center (Transformation|GetActorLocation) :Extent (Math|Vector|MakeVector (Math|Conversions|ToFloat(Integer) (* (Variables|Default|GetBuildingX) (/ _tilesize 2))) (Math|Conversions|ToFloat(Integer) (* (/ _tilesize 2) (Variables|Default|GetBuildingY))) 2e+01)))