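; First-person player character Blueprint that creates the main HUD on begin play and handles firing at enemies.
; Fire input runs a short debug-drawn visibility line trace forward from the first-person camera.
; A hit on an EnemyCharacter is cast to EnemyCharacter_BP and reported dead immediately, with no damage step.
; A weapon mesh attachment to the arms socket exists but is disconnected, so it never runs.
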(event EventBeginPlay
  (bind _returnvalue (UserInterface|CreateWidget "/Game/UI/MainHUD_Widget.MainHUD_Widget_C"))
  (UserInterface|Viewport|AddtoViewport _returnvalue 0))

(event Collision|EventActorBeginOverlap
  (params (OtherActor :type Actor%20Object%20Reference)))

(event EventTick
  (params (DeltaSeconds :type Float%20%28single-precision%29)))

(event Input|ActionEvents|InputActionFire
  (params (Key :type Key%20Structure :default "None"))
  (bind _firstpersoncameracomponent (Variables|Default|GetFirstPersonCameraComponent))
  (bind _returnvalue (Transformation|GetWorldLocation _firstpersoncameracomponent))
  (:Pressed
    (bind _outhit (Collision|LineTraceByChannel _returnvalue (+ _returnvalue (* (Math|Vector|GetForwardVector (Transformation|GetWorldRotation _firstpersoncameracomponent)) 1000)) "TraceTypeQuery1" false 0 "ForOneFrame"))
    (if (Utilities|ClassIsChildOf (Utilities|GetClass (.hitactor _outhit)) "/Script/Hoard.EnemyCharacter")
      (bind _asenemy_character_bp (Utilities|Casting|CastToEnemyCharacter_BP (.hitactor _outhit)))
      (Default|ReportDeath _asenemy_character_bp))))

(fn ConstructionScript)